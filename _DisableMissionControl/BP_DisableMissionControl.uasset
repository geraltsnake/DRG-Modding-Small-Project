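; BP_DisableMissionControl is a mod actor that silences Mission Control for the local player.
; On BeginPlay it retries every three seconds until the local player character and FSD player controller are valid.
; It then pauses Mission Control through the character's CommunicationComponent.
; Several leftover sound and shout nodes are disconnected and never run.
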(event EventBeginPlay
  (bind _returnvalue (Game|GetGameInstance))
  (bind _returnvalue_2 (Class|GameFunctionLibrary|GetFSDGameInstance _returnvalue))
  (bind _returnvalue_3 (Class|GameFunctionLibrary|GetLocalPlayerCharacter _returnvalue_2))
  (if (and (Utilities|IsValid _returnvalue_3) (Utilities|IsValid (Class|FSDGameInstance|GetLocalFSDPlayerController _returnvalue_2))) :!label _label
    (Class|CommunicationComponent|SetMissionControlPaused (Variables|/Script/FSD.PlayerCharacter|GetCommunicationComponent _returnvalue_3) true)
    (else
      (Utilities|FlowControl|Delay 3.0)
      (goto _label))))

(fn ConstructionScript)